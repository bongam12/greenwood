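; AI controller for base enemies that runs their behavior tree and targets the player.
; On possess it waits ten seconds, starts BT_BaseEnemy, then sets the player character as the Blackboard's AttackTarget.
; BeginPlay gathers all actors and those tagged EnemyCover, but the distance-based cover selection and debug prints are disconnected and never run.
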(event `self.ReceivePossess`
  (params (PossessedPawn :type "Pawn Object Reference"))
  (`KismetSystemLibrary.Delay` 10.0)
  (`self.RunBehaviorTree` "/Game/Custom_BPs/enemies/AI/BT_BaseEnemy.BT_BaseEnemy")
  (`BlackboardComponent.SetValueAsObject` (`self.Blackboard`) (`self.AttackTarget`) (`GameplayStatics.GetPlayerCharacter` 0)))

(event `self.ReceiveBeginPlay`
  (bind _outactors (`GameplayStatics.GetAllActorsOfClass` "/Script/Engine.Actor"))
  (bind _outactors_2 (`GameplayStatics.GetAllActorsWithTag` "EnemyCover")))

(fn `UserConstructionScript`)